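; Traffic light head Blueprint for a CARLA scenario that shows the current signal state on its red, yellow and green lamp meshes.
; On a state change it swaps each lamp's material, lighting the active one through an "On/Off" scalar parameter and darkening the others, or all three when Off.
; It then notifies every vehicle in StoppedCars.
; GetTriggerVolume returns no volume and the construction script is empty.
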(event `self.OnTrafficLightStateChanged`
  (params (TrafficLightState :type "ETrafficLightState Enum" :default "Red"))
  (bind _yellowlight (`self.YellowLight`))
  (bind _greenlight (`self.GreenLight`))
  (bind _redlight (`self.RedLight`))
  (`|ExecutionSequence`
    (:`then_0`
      (switch `ETrafficLightState` TrafficLightState
        (:`Red`
          (`PrimitiveComponent.SetMaterial` _redlight 1 "/Game/Carla/Static/TrafficLight/Streetlights_01/MI_Streetlights_2.MI_Streetlights_2")
          (`MeshComponent.SetScalarParameterValueOnMaterials` _redlight "On/Off" 1.0)
          (`PrimitiveComponent.SetMaterial` (`self.YellowLight`) 1 "/Game/Carla/Static/TrafficLight/Streetlights_01/MI_StreetLightsOff.MI_StreetLightsOff")
          (`PrimitiveComponent.SetMaterial` (`self.GreenLight`) 1 "/Game/Carla/Static/TrafficLight/Streetlights_01/MI_StreetLightsOff.MI_StreetLightsOff"))
        (:`Yellow`
          (`PrimitiveComponent.SetMaterial` (`self.RedLight`) 1 "/Game/Carla/Static/TrafficLight/Streetlights_01/MI_StreetLightsOff.MI_StreetLightsOff")
          (`PrimitiveComponent.SetMaterial` _yellowlight 1 "/Game/Carla/Static/TrafficLight/Streetlights_01/MI_Streetlights_1.MI_Streetlights_1")
          (`MeshComponent.SetScalarParameterValueOnMaterials` _yellowlight "On/Off" 1.0)
          (`PrimitiveComponent.SetMaterial` (`self.GreenLight`) 1 "/Game/Carla/Static/TrafficLight/Streetlights_01/MI_StreetLightsOff.MI_StreetLightsOff"))
        (:`Green`
          (`PrimitiveComponent.SetMaterial` (`self.RedLight`) 1 "/Game/Carla/Static/TrafficLight/Streetlights_01/MI_StreetLightsOff.MI_StreetLightsOff")
          (`PrimitiveComponent.SetMaterial` (`self.YellowLight`) 1 "/Game/Carla/Static/TrafficLight/Streetlights_01/MI_StreetLightsOff.MI_StreetLightsOff")
          (`PrimitiveComponent.SetMaterial` _greenlight 1 "/Game/Carla/Static/TrafficLight/Streetlights_01/MI_Streetlights_3.MI_Streetlights_3")
          (`MeshComponent.SetScalarParameterValueOnMaterials` _greenlight "On/Off" 1.0))
        (:`Off`
          (`PrimitiveComponent.SetMaterial` (`self.RedLight`) 1 "/Game/Carla/Static/TrafficLight/Streetlights_01/MI_StreetLightsOff.MI_StreetLightsOff")
          (`PrimitiveComponent.SetMaterial` (`self.YellowLight`) 1 "/Game/Carla/Static/TrafficLight/Streetlights_01/MI_StreetLightsOff.MI_StreetLightsOff")
          (`PrimitiveComponent.SetMaterial` (`self.GreenLight`) 1 "/Game/Carla/Static/TrafficLight/Streetlights_01/MI_StreetLightsOff.MI_StreetLightsOff"))))
    (:`then_1`
      (for _array_element (`self.StoppedCars`)
        (`self.NotifyWheeledVehicle` _array_element)))))

(fn `GetTriggerVolume`
  (returns (ReturnValue :type "BoxComponent Object Reference"))
  (return null))

(fn `UserConstructionScript`)